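; DreamBisky is the playable Bisky character, with movement relative to control yaw and an E key interaction.
; While IsPushing is set, movement is locked to the forward or sideways axis by comparing PushDirection to a text label.
; Setter functions expose both push values.
; Pressing E sends an Interact message, passing itself, to the first actor overlapping the capsule, with no check for an empty list.
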(event `InputAxis|MoveRight`
  (params (AxisValue :type "Float (single-precision)"))
  ;[1 1 1] Movement
  (if (`self.IsPushing`)
    (if (`KismetTextLibrary.EqualEqual_TextText` (`self.Push direction`) "sideways")
      (`self.AddMovementInput` (`KismetMathLibrary.GetRightVector` (`KismetMathLibrary.MakeRotator` 0.0 0.0 (.yaw (`self.GetControlRotation`)))) AxisValue :!label _label))
    (else
      (goto _label))))

(event `InputAxis|MoveForward`
  (params (AxisValue :type "Float (single-precision)"))
  ;[1 1 1] Movement
  (if (`self.IsPushing`)
    (if (`KismetTextLibrary.EqualEqual_TextText` (`self.Push direction`) "forward")
      (`self.AddMovementInput` (`KismetMathLibrary.GetForwardVector` (`KismetMathLibrary.MakeRotator` 0.0 0.0 (.yaw (`self.GetControlRotation`)))) AxisValue :!label _label_2))
    (else
      (goto _label_2))))

(event `Key|E`
  (params (Key :type "Key Structure"))
  ;[1 1 1] Press E to interact on Actors Bisky is overlapping
  (:`Pressed`
    (message `/Game/DoggyGame/Blueprints/BiskInterface.Interact` (`|GetArrayItem` (`PrimitiveComponent.GetOverlappingActors` (`self.CapsuleComponent`) null)) self)))

(fn `Set Push Direction`
  (params (NewParam :type Text))
  (set `self.Push direction` NewParam))

(fn `SetIsPushing`
  (params (`bool isBiskyPushing` :type Boolean))
  (set `self.IsPushing` `bool isBiskyPushing`))

(fn `UserConstructionScript`)