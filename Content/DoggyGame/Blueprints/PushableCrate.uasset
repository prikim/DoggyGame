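; Pushable crate actor that Bisky grabs and releases through the Interact event.
; Interact casts to DreamBisky and calls PushCrate, which flips IsBeingPushed, passes it to Bisky via SetIsPushing, and attaches or detaches the crate, keeping world transform.
; Movement comes entirely from attachment: tick is disabled at BeginPlay, and an interpolated follow-in-front-of-Bisky block is left unconnected.
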(event `self.ReceiveBeginPlay`
  ;[1 1 1] Initialize
  (`self.SetActorTickEnabled` false))

(event `/Game/DoggyGame/Blueprints/BiskInterface.Interact`
  (params (Bisky :type "Actor Object Reference"))
  (bind _asdream_bisky (cast `/Game/DoggyGame/Blueprints/DreamBisky` Bisky)
    (:`then`
      (`self.PushCrate` _asdream_bisky) ; enables and disables ticking when Bisky is interacting
    )
    (:`CastFailed`
      (`KismetSystemLibrary.PrintString` "cast to dreambisky failed from pushable crate"))))

(event `self.ReceiveTick`
  (params (DeltaSeconds :type "Float (single-precision)")))

(fn `PushCrate`
  (params (Bisky :type "/Game/DoggyGame/Blueprints/DreamBisky Object Reference"))
  (locals (`DreamBisky Ref` :type "/Game/DoggyGame/Blueprints/DreamBisky Object Reference"))
  (bind _isbeingpushed (`self.IsBeingPushed`))
  (bind _dreambisky_ref (`local.DreamBisky Ref`))
  (bind _returnvalue (not _isbeingpushed))
  (set `local.DreamBisky Ref` Bisky)
  (if _isbeingpushed
    ;[1 1 1] Crate is not being pushed
    (bind _output_get (set `self.IsBeingPushed` _returnvalue))
    (`/Game/DoggyGame/Blueprints/DreamBisky.SetIsPushing` _dreambisky_ref _output_get)
    (`KismetSystemLibrary.PrintString` "Crate immovable")
    (`self.K2_DetachFromActor` "KeepWorld" "KeepWorld" "KeepWorld")
    (else
      ;[1 1 1] Crate is being pushed
      (bind _output_get_2 (set `self.IsBeingPushed` _returnvalue))
      (`/Game/DoggyGame/Blueprints/DreamBisky.SetIsPushing` _dreambisky_ref _output_get_2)
      (`KismetSystemLibrary.PrintString` "Moving Crate")
      (`self.K2_AttachToActor` _dreambisky_ref "None" "KeepWorld" "KeepWorld" "KeepWorld"))))

(fn `UserConstructionScript`)