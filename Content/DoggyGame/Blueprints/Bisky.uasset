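; Bisky is a playable Character Blueprint with camera-relative movement, camera look and jumping.
; Movement input follows the controller's yaw only, while camera axes drive controller yaw and pitch.
; Pressing E sends InteractMessage to the first actor overlapping the capsule.
; Overlapping a Bed prints an on-screen "press e" prompt through PrintString.
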(event `self.ReceiveBeginPlay`)

(event `InputAxis|MoveRight`
  (params (AxisValue :type "Float (single-precision)"))
  ;[1 1 1] 3D movement
  (`self.AddMovementInput` (`KismetMathLibrary.GetRightVector` (`KismetMathLibrary.MakeRotator` 0.0 0.0 (.yaw (`self.GetControlRotation`)))) AxisValue))

(event `InputAxis|CameraX`
  (params (AxisValue :type "Float (single-precision)"))
  ;[1 1 1] Camera
  (`self.AddControllerYawInput` AxisValue))

(event `InputAction|Jump`
  (params (Key :type "Key Structure"))
  (:`Pressed`
    (`self.Jump`)))

(event `InputAxis|CameraY`
  (params (AxisValue :type "Float (single-precision)"))
  ;[1 1 1] Camera
  (`self.AddControllerPitchInput` AxisValue))

(event `InputAxis|MoveForward`
  (params (AxisValue :type "Float (single-precision)"))
  ;[1 1 1] 3D movement
  (`self.AddMovementInput` (`KismetMathLibrary.GetForwardVector` (`KismetMathLibrary.MakeRotator` 0.0 0.0 (.yaw (`self.GetControlRotation`)))) AxisValue))

(event `Key|E`
  (params (Key :type "Key Structure"))
  ;[1 1 1] Press E to interact on Actors Bisky is overlapping
  (:`Pressed`
    (message `/Game/DoggyGame/Blueprints/BiskInterface.Interact` (`|GetArrayItem` (`PrimitiveComponent.GetOverlappingActors` (`self.CapsuleComponent`) null)) null)))

(event `self.ReceiveActorBeginOverlap`
  (params (OtherActor :type "Actor Object Reference"))
  ;[1 1 1] Prompt for Bisky
  (cast `/Game/DoggyGame/Blueprints/Bed` OtherActor)
  (if true
    (`KismetSystemLibrary.PrintString` "press e")))

(fn `UserConstructionScript`)